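; BP_HUD_Game is the HUD for the 3D runner, managing the main menu, in-game HUD and game over screens.
; On BeginPlay it creates and stores all three widgets, shows only the main menu and sets Game and UI input.
; Interface events ToGameStart and ToGameOver call functions that add the game HUD, then later replace it with the game over screen.
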(event EventBeginPlay
  (bind _returnvalue (UserInterface|CreateWidget "/Game/3DRunner/UI/WBP_MainMenu.WBP_MainMenu_C" (Game|Player|GetOwningPlayerController)))
  (bind _output_get (Variables|Default|SetWBP%20Main%20Menu _returnvalue))
  (UserInterface|Viewport|AddtoViewport _output_get 0)
  (Input|SetInputModeGameandUI (Game|Player|GetOwningPlayerController) 0 "DoNotLock" false false)
  (bind _returnvalue_2 (UserInterface|CreateWidget "/Game/3DRunner/UI/WBP_GameOver.WBP_GameOver_C" (Game|Player|GetOwningPlayerController)))
  (Variables|Default|SetWBP%20Game%20Over _returnvalue_2)
  (bind _returnvalue_3 (UserInterface|CreateWidget "/Game/3DRunner/UI/WBP_GameHUD.WBP_GameHUD_C" (Game|Player|GetOwningPlayerController)))
  (Variables|Default|SetWBP%20Game%20HUD _returnvalue_3))

(event EventToGameStart
  ;[1 1 1] Event Interface for Game Start and Over
  (CallFunction|GameStart))

(event EventToGameOver
  ;[1 1 1] Event Interface for Game Start and Over
  (CallFunction|GameOver))

(fn ConstructionScript)

(fn GameOver
  (UserInterface|Viewport|AddtoViewport (Variables|Default|GetWBP%20Game%20Over) 0)
  (Widget|RemovefromParent (Variables|Default|GetWBP%20Game%20HUD)))

(fn GameStart
  (UserInterface|Viewport|AddtoViewport (Variables|Default|GetWBP%20Game%20HUD) 0))