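; Floor tile actor for a 3D runner that fills itself with random obstacles and trees.
; The construction script creates one spawn point per lane at a random forward offset, then shuffles them to place randomly picked obstacle child actors, leaving some empty.
; Tree points each get one of two child actor variants with random yaw.
; Overlapping the end box tells the game mode to spawn the next floors, while GetSpawnPoint exposes the tile's attachment transform.
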(event OnComponentBeginOverlap(EndBox)
  (params (OverlappedComponent :type Primitive%20Component%20Object%20Reference) (OtherActor :type Actor%20Object%20Reference) (OtherComp :type Primitive%20Component%20Object%20Reference) (OtherBodyIndex :type Integer) (bFromSweep :type Boolean) (SweepResult :type Hit%20Result%20Structure%20%28by%20ref%29))
  ;[1 1 1] On Overlap - Spawn Next Floors in Game Mode
  (bind _asrunner_game_game_mode (Utilities|Casting|CastToRunnerGameGameMode (Game|GetGameMode)))
  (Class|RunnerGameGameMode|SpawnNextFloors _asrunner_game_game_mode))

(fn ConstructionScript
  (CallFunction|InitSpawnPoints)
  (CallFunction|SpawnObstacles)
  (CallFunction|SpawnTrees))

(fn GetSpawnPoint
  (return (Transformation|GetWorldTransform (Variables|Default|GetSpawnPoint))))

(fn InitSpawnPoints
  (for _array_element (Variables|Default|GetLane%20Positions)
    (bind _returnvalue (AddComponent|AddArrowComponent false (Math|Transform|MakeTransform (Math|Vector|MakeVector (Math|Random|RandomFloatinRange 2.5e+02 1.75e+03) _array_element 0.0))))
    (Utilities|Array|Add (Variables|Default|GetSpawn%20Points) (Transformation|GetWorldTransform _returnvalue))))

(fn SpawnObstacles
  (bind _output_get (LocalVariables|SetRandom%20Spawn%20Points (Variables|Default|GetSpawn%20Points)))
  (Utilities|Array|Shuffle _output_get)
  (for _index (range 0 (Math|Random|RandomIntegerinRange 1 2))
    (switch int (Math|Random|RandomIntegerinRange 0 5)
      (:0
        (AddComponent|AddChildActorComponent false (Math|Transform|MakeRelativeTransform (Utilities|Array|Get(acopy) (LocalVariables|GetRandom%20Spawn%20Points) _index) (Transformation|GetActorTransform))))
      (:1
        (AddComponent|AddChildActorComponent false (Math|Transform|MakeRelativeTransform (Utilities|Array|Get(acopy) (LocalVariables|GetRandom%20Spawn%20Points) _index) (Transformation|GetActorTransform))))
      (:2
        (AddComponent|AddChildActorComponent false (Math|Transform|MakeRelativeTransform (Utilities|Array|Get(acopy) (LocalVariables|GetRandom%20Spawn%20Points) _index) (Transformation|GetActorTransform))))
      (:3
        (AddComponent|AddChildActorComponent false (Math|Transform|MakeRelativeTransform (Utilities|Array|Get(acopy) (LocalVariables|GetRandom%20Spawn%20Points) _index) (Transformation|GetActorTransform)))))))

(fn SpawnTrees
  (for _array_element (Variables|Default|GetTree%20Spawn%20Points)
    (switch int (Math|Random|RandomIntegerinRange 0 1)
      (:0
        (bind _returnvalue (AddComponent|AddChildActorComponent false _array_element))
        (Transformation|SetRelativeRotation _returnvalue (Math|Rotator|MakeRotator 0.0 0.0 (Math|Random|RandomFloatinRange 0.0 3.6e+02)) false false))
      (:1
        (bind _returnvalue_2 (AddComponent|AddChildActorComponent false _array_element))
        (Transformation|SetRelativeRotation _returnvalue_2 (Math|Rotator|MakeRotator 0.0 0.0 (Math|Random|RandomFloatinRange 0.0 3.6e+02)) false false)))))