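; Player character for a 3D runner that switches between three lanes, jumps and tracks distance travelled.
; Touch swipes or A, D and Space drive movement, with a timeline interpolating Y between lane positions.
; Ability interface events trigger a timed sprint with Niagara effect or a swept forward teleport.
; A self-calling Delay loop accumulates distance, which passes to BP_PC_Game on unpossess before the character destroys itself.
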(event Custom|MoveLeftRight
  (params (Change%20Lane :type Integer))
  (bind _returnvalue (Transformation|GetActorLocation))
  ;[1 1 1] Move Character Left or Right
  (Variables|Move|SetTarget%20Lane%20Index (Math|Integer|Clamp(Integer) (+ Change%20Lane (Variables|Move|GetCurrent%20Lane%20Index)) 0 2))
  (Variables|Move|SetCurrent%20Y%20Pos (.y (Transformation|GetActorLocation)))
  (bind _change (Timeline|Change%20Lane PlayFromStart)
    (:Update
      (Transformation|SetActorLocation (Math|Vector|MakeVector (.x _returnvalue) (Math|Float|Lerp (Variables|Move|GetCurrent%20Y%20Pos) (Utilities|Array|Get(acopy) (Variables|Move|GetLane%20Positions) (Variables|Move|GetTarget%20Lane%20Index)) _change) (.z _returnvalue)) false false))
    (:Finished
      (Variables|Move|SetCurrent%20Lane%20Index (Variables|Move|GetTarget%20Lane%20Index)))))

(event Custom|Touch%20Input
  (bind _returnvalue (Game|GetPlayerController 0))
  (bind (_locationx _locationy) (Class|PlayerController|GetInputTouchState _returnvalue "Touch1"))
  (if (> (Math|Vector2D|Vector2DLength (- (Variables|TouchInput|GetTouch%20Start) (Variables|TouchInput|GetTouch%20End))) 1e+02)
    (Utilities|FlowControl|DoOnce false
      (:Completed
        (Variables|TouchInput|SetTouch%20End (Math|Vector2D|MakeVector2D _locationx _locationy))
        (if (> (Math|Float|Absolute(Float) (.x (- (Variables|TouchInput|GetTouch%20Start) (Variables|TouchInput|GetTouch%20End)))) (Math|Float|Absolute(Float) (.y (- (Variables|TouchInput|GetTouch%20Start) (Variables|TouchInput|GetTouch%20End)))))
          (if (> (.x (- (Variables|TouchInput|GetTouch%20Start) (Variables|TouchInput|GetTouch%20End))) 0.0)
            (Development|PrintString "Left")
            (CallFunction|MoveLeftRight -1)
            (else
              (Development|PrintString "Right")
              (CallFunction|MoveLeftRight 1)))
          (elif (> (.y (- (Variables|TouchInput|GetTouch%20Start) (Variables|TouchInput|GetTouch%20End))) 0.0)
            (Development|PrintString "Up")
            (Character|Jump)
            (else
              (Development|PrintString "Down"))))))))

(event EventTeleport
  ;[1 1 1] Event Teleport
  (Transformation|SetActorLocation (+ (* (Transformation|GetActorForwardVector) 1000) (Transformation|GetActorLocation)) true false))

(event EventBeginPlay
  ;[1 1 1] Event on Being Play
  (Variables|Distance|SetLocation (Transformation|GetActorLocation))
  (Class|RunnerGameCharacter|FindDistance)
  (Components|Activation|Deactivate (Variables|Default|GetNiagara)))

(event EventTick
  (params (DeltaSeconds :type Float%20%28single-precision%29))
  (if (Variables|TouchInput|GetIs%20Pressed)
    (CallFunction|TouchInput)))

(event EventStartSprinting
  ;[1 1 1] Event Start Sprinting and Stop Sprinting after 5 Seconds
  (Variables|/Script/Engine.CharacterMovementComponent|SetMaxWalkSpeed (Variables|Character|GetCharacterMovement) 2e+03)
  (bind _returnvalue (Utilities|Time|SetTimerbyEvent (delegate EventStopSprinting) 5.0))
  (Variables|Sprint|SetTimer%20Handle _returnvalue)
  (Components|Activation|Activate (Variables|Default|GetNiagara) false))

(event EventStopSprinting
  ;[1 1 1] Event Start Sprinting and Stop Sprinting after 5 Seconds
  (Variables|/Script/Engine.CharacterMovementComponent|SetMaxWalkSpeed (Variables|Character|GetCharacterMovement) 1e+03)
  (Utilities|Time|ClearandInvalidateTimerbyHandle (Variables|Sprint|GetTimer%20Handle))
  (Components|Activation|Deactivate (Variables|Default|GetNiagara)))

(event EventFindDistance
  ;[1 1 1] Event Find Distance travelled by Character
  (Variables|Distance|SetDistance%20Travelled (+ (Math|Vector|VectorLength (- (Variables|Distance|GetLocation) (Transformation|GetActorLocation))) (Variables|Distance|GetDistance%20Travelled)))
  (Variables|Distance|SetLocation (Transformation|GetActorLocation))
  (Utilities|FlowControl|Delay 0.001)
  (Class|RunnerGameCharacter|FindDistance))

(event EventToSprint
  ;[1 1 1] Character Ability Interface Functions
  (Class|RunnerGameCharacter|StartSprinting))

(event EventToTeleport
  ;[1 1 1] Character Ability Interface Functions
  (Class|RunnerGameCharacter|Teleport))

(event EventUnpossessed
  (params (OldController :type Controller%20Object%20Reference))
  ;[1 1 1] Event On Unpossessed
  (bind _asbp_pc_game (Utilities|Casting|CastToBP_PC_Game OldController))
  (Default|SetDistance _asbp_pc_game (Variables|Distance|GetDistance%20Travelled))
  (Actor|DestroyActor))

(event Input|KeyboardEvents|A
  (params (Key :type Key%20Structure :default "None"))
  ;[1 1 1] Keyboard Button
  (:Pressed
    (CallFunction|MoveLeftRight -1)))

(event Input|KeyboardEvents|D
  (params (Key :type Key%20Structure :default "None"))
  ;[1 1 1] Keyboard Button
  (:Pressed
    (CallFunction|MoveLeftRight 1)))

(event Input|KeyboardEvents|SpaceBar
  (params (Key :type Key%20Structure :default "None"))
  ;[1 1 1] Keyboard Button
  (:Pressed
    (Character|Jump)))

(event Input|TouchEvents|InputTouch
  (params (Location :type Vector) (FingerIndex :type ETouchIndex%20Enum))
  (bind _returnvalue (Game|GetPlayerController 0))
  (bind (_locationx _locationy) (Class|PlayerController|GetInputTouchState _returnvalue "Touch1"))
  (:Pressed
    (Variables|TouchInput|SetIs%20Pressed true)
    (Variables|TouchInput|SetTouch%20Start (Math|Vector2D|MakeVector2D (.x Location) (.y Location))))
  (:Released
    (Variables|TouchInput|SetTouch%20End (Math|Vector2D|MakeVector2D (.x Location) (.y Location)))
    (Utilities|FlowControl|DoOnce false) ; enters at Reset
  ))

(fn ConstructionScript)