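; Game mode for a 3D runner that spawns and possesses the player, runs a countdown timer and handles game over and restart.
; Floor actors chain from each previous floor's spawn point, and spawning a next floor destroys the oldest once more than 12 exist.
; Each Tick takes one second off the timer; at zero the player is unpossessed, the HUD is notified and the timer resets.
; Restart clears the floors, respawns the initial set and starts a new game.
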(event EventStartGame
  (CallFunction|SpawnPlayer)
  (Variables|Default|SetIs%20Game%20Started true))

(event EventRestartGame
  (bind _floors (Variables|GameMode|GetFloors))
  ;[1 1 1] Event Restart Game
  (for (_array_element _array_index) _floors
    (Actor|DestroyActor _array_element)
    (Utilities|Array|RemoveIndex _floors _array_index))
  (Variables|GameMode|SetFloor%20Spawn%20Point "")
  (for _index (range 0 (Variables|Default|GetNumOfInitialFloors))
    (Class|RunnerGameGameMode|SpawnFirstFloors))
  (Class|RunnerGameGameMode|StartGame))

(event EventSpawnFirstFloors
  ;[1 1 1] Event Spawn First Initital Floors
  (bind _returnvalue (Game|SpawnActorfromClass "/Game/3DRunner/Blueprints/Actors/AC_BaseFloor.AC_BaseFloor_C" (Variables|GameMode|GetFloor%20Spawn%20Point) "Undefined" 0 0))
  (Variables|GameMode|SetFloor%20Spawn%20Point (Default|GetSpawnPoint _returnvalue))
  (Utilities|Array|Add (Variables|GameMode|GetFloors) _returnvalue))

(event EventSpawnNextFloors
  (bind _floors (Variables|GameMode|GetFloors))
  ;[1 1 1] Event Spawn Next Floors
  (Class|RunnerGameGameMode|SpawnFirstFloors)
  (if (> (Utilities|Array|Length (Variables|GameMode|GetFloors)) 12)
    (Actor|DestroyActor (Utilities|Array|Get(acopy) _floors))
    (Utilities|Array|RemoveIndex _floors)))

(event EventGameOver
  (bind _returnvalue (Game|GetPlayerController 0))
  ;[1 1 1] Event Game Over
  (Pawn|UnPossess _returnvalue)
  (Class|BPIHUDEvents|ToGameOver(Message) (HUD|GetHUD _returnvalue))
  (Variables|Default|SetMinutes 3)
  (Variables|Default|SetSeconds 0)
  (Variables|Default|SetIs%20Game%20Started false))

(event EventTick
  (params (DeltaSeconds :type Float%20%28single-precision%29))
  (if (Variables|Default|GetIs%20Game%20Started)
    (if (== (Variables|Default|GetSeconds) 0)
      (if (== (Variables|Default|GetMinutes) 0)
        (Class|RunnerGameGameMode|GameOver)
        (else
          (Variables|Default|SetSeconds 59)
          (Variables|Default|SetMinutes (- (Variables|Default|GetMinutes) 1))))
      (else
        (Variables|Default|SetSeconds (- (Variables|Default|GetSeconds) 1))))))

(fn ConstructionScript)

(fn SpawnPlayer
  (bind _returnvalue (Game|GetPlayerController 0))
  (bind _returnvalue_2 (Game|SpawnActorfromClass "/Game/3DRunner/Blueprints/Characters/BP_C_GameCharacter.BP_C_GameCharacter_C" (CallFunction|GetPlayerStart) "Undefined" (Game|GetPlayerController 0) 0))
  (Pawn|Possess _returnvalue _returnvalue_2)
  (Class|BPIHUDEvents|ToGameStart(Message) (HUD|GetHUD _returnvalue)))

(fn GetPlayerStart
  (bind _returnvalue (Actor|GetActorOfClass "/Script/Engine.PlayerStart"))
  (return (Transformation|GetActorTransform _returnvalue)))